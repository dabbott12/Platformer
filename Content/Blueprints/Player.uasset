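; Player pawn that moves on axis input, jumps, tracks score and handles game over.
; Movement uses actor-relative movement input, while jumping applies a mass-independent upward force to the static mesh, gated by a Grounded flag that near-exact upward hit normals restore.
; It creates the game HUD on BeginPlay and pushes score changes to it.
; GameOver shows the end screen, enables the mouse cursor and pauses the game.
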(event `InputAction|Jump`
  (params (Key :type "Key Structure"))
  ;[1 1 1] Jumping
  (:`Pressed`
    (if (`self.Grounded`)
      (`PrimitiveComponent.AddForce` (`self.StaticMesh`) (* (`KismetMathLibrary.Vector_Up`) (`self.JumpForce`)) "None" true)
      (set `self.Grounded` false))))

(event `InputAxis|Move_ForwardBack`
  (params (AxisValue :type "Float (single-precision)"))
  ;[1 1 1] Movement
  (`self.AddMovementInput` (`self.GetActorForwardVector`) AxisValue))

(event `InputAxis|Move_LeftRight`
  (params (AxisValue :type "Float (single-precision)"))
  ;[1 1 1] Movement
  (`self.AddMovementInput` (`self.GetActorRightVector`) AxisValue))

(event `self.ReceiveHit`
  (params (MyComp :type "PrimitiveComponent Object Reference") (Other :type "Actor Object Reference") (OtherComp :type "PrimitiveComponent Object Reference") (bSelfMoved :type Boolean) (HitLocation :type "Vector Structure") (HitNormal :type "Vector Structure") (NormalImpulse :type "Vector Structure") (Hit :type "HitResult Structure (by ref)"))
  ;[1 1 1] Grounded Check
  (if (== HitNormal (`KismetMathLibrary.Vector_Up`) :`ErrorTolerance` 1e-06)
    (set `self.Grounded` true)))

(event `self.ReceiveBeginPlay`
  ;[1 1 1] UI
  (bind _returnvalue (`|CreateWidget` "/Game/Blueprints/GameUI.GameUI_C"))
  (`UserWidget.AddToViewport` _returnvalue 0)
  (set `self.GameUI` _returnvalue))

(fn `AddScore`
  (params (ScoreToAdd :type Integer))
  (bind _output_get (set `self.Score` (+ ScoreToAdd (`self.Score`))))
  (`/Game/Blueprints/GameUI.SetScore` (`self.GameUI`) _output_get))

(fn `GameOver`
  ;[1 1 1] GameOver Function - With Menu
  (bind _returnvalue (`|CreateWidget` "/Game/Blueprints/EndGameUI.EndGameUI_C"))
  (`UserWidget.AddToViewport` _returnvalue 0)
  (`/Game/Blueprints/EndGameUI.SetEndScreen` _returnvalue false)
  (bind _output_get (set `PlayerController.bShowMouseCursor` true (`GameplayStatics.GetPlayerController` 0)))
  (`GameplayStatics.SetGamePaused` _output_get))

(fn `UserConstructionScript`)